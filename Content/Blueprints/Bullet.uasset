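; Bullet is a projectile actor that flies in a straight line to a destination point and then destroys itself.
; SetActor stores the owning character and sets the destination from the bullet's forward vector and that character's Range.
; On authority only, Tick teleports it Speed units per frame without sweep or delta-time scaling, destroying it once within Speed on every axis.
; The graphs contain no hit or damage logic.
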(event EventTick
  (params (DeltaSeconds :type Float%20%28single-precision%29))
  (bind _returnvalue (Transformation|GetActorLocation))
  (bind _returnvalue_2 (Transformation|GetActorLocation))
  (bind _speed (Variables|Default|Getspeed))
  (bind _dest (Variables|Default|Getdest))
  (bind _returnvalue_3 (- _returnvalue_2 _dest))
  (bind (_x _y _z) (Math|Vector|BreakVector _returnvalue_3))
  (Networking|SwitchHasAuthority
    (:Authority
      (Transformation|SetActorLocation (+ (* (Math|Vector|Normalize (- (Variables|Default|Getdest) _returnvalue)) _speed) _returnvalue) false)
      (if (and (and (<= (Math|Float|Absolute(Float) _x) _speed) (<= (Math|Float|Absolute(Float) _y) _speed)) (<= (Math|Float|Absolute(Float) _z) _speed))
        (Actor|DestroyActor)))))

(fn ConstructionScript)

(fn SetActor
  (params (Character :type My%20Character%20Object%20Reference))
  (Variables|Default|SetOwner_actor Character)
  (Variables|Default|Setdest (+ (* (Transformation|GetActorForwardVector) (Variables|/Game/Blueprints/MyCharacter.MyCharacter_C|Getrange (Variables|Default|GetOwner_actor))) (Transformation|GetActorLocation))))